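; BP_Ghost is a monster character whose death sound depends on its Level value, with mesh, life and walk speed initialized only for WHITE.
; Damage lowers Life by whole numbers; at zero it waits briefly, plays the sound and destroys itself.
; Touching the player calls GetDamage on MyGameMode, while projectile hits briefly halt it, then set a walk speed faster than the WHITE starting one.
; SetMode's switch has no branch logic.
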(event EventBeginPlay
  (if (Utilities|Enum|Equal(Enum) (Variables|Default|Getlevel) "WHITE")
    (CallFunction|SetWhiteMesh)
    (Variables|Default|Setlife 3)
    (Variables|/Script/Engine.CharacterMovementComponent|SetMaxWalkSpeed (Variables|Character|GetCharacterMovement) 2e+02)))

(event Game|Damage|EventAnyDamage
  (params (Damage :type Float%20%28single-precision%29) (DamageType :type Damage%20Type%20Object%20Reference) (InstigatedBy :type Controller%20Object%20Reference) (DamageCauser :type Actor%20Object%20Reference))
  (Development|PrintText "아프다")
  (bind _output_get (Variables|Default|Setlife (- (Variables|Default|Getlife) (Math|Float|Truncate Damage))))
  (if (<= _output_get 0)
    (Utilities|FlowControl|Delay 0.2)
    (CallFunction|PlayDeathSound)
    (Actor|DestroyActor)))

(event Collision|EventHit
  (params (MyComp :type Primitive%20Component%20Object%20Reference) (Other :type Actor%20Object%20Reference) (OtherComp :type Primitive%20Component%20Object%20Reference) (bSelfMoved :type Boolean) (HitLocation :type Vector :default "0, 0, 0") (HitNormal :type Vector :default "0, 0, 0") (NormalImpulse :type Vector :default "0, 0, 0") (Hit :type Hit%20Result%20Structure%20%28by%20ref%29))
  (bind _charactermovement (Variables|Character|GetCharacterMovement))
  (Utilities|Casting|CastToFirstPersonCharacter Other
    (:then
      (bind _asmy_game_mode (Utilities|Casting|CastToMyGameMode (Game|GetGameMode)))
      (Default|GetDamage _asmy_game_mode 0.01))
    (:CastFailed
      (Utilities|Casting|CastToFirstPersonProjectile Other)
      (Variables|/Script/Engine.CharacterMovementComponent|SetMaxWalkSpeed _charactermovement 0.0)
      (Utilities|FlowControl|Delay 0.3)
      (Variables|/Script/Engine.CharacterMovementComponent|SetMaxWalkSpeed _charactermovement 6e+02))))

(fn ConstructionScript)

(fn SetMode
  (params (mode :type Integer))
  (bind _output_get (Variables|Default|Setmode mode))
  (switch int _output_get))

(fn SetWhiteMesh
  (bind _staticmesh (Variables|Default|GetStaticMesh))
  (Components|StaticMesh|SetStaticMesh _staticmesh "/Game/Monster/ghost_assets/ghost_FINAL.ghost_FINAL")
  (Rendering|Material|SetMaterial _staticmesh 0 "/Game/Monster/ghost_assets/ghost_Opacity_Mat.ghost_Opacity_Mat")
  (Class|SkinnedMeshComponent|SetSkeletalMesh (Variables|Character|GetMesh) 0 true))

(fn PlayDeathSound
  (if (Utilities|Enum|Equal(Enum) (Variables|Default|Getlevel) "BLACK")
    (Audio|PlaySound2D "/Game/Audio/black_death.black_death" 1.0 1.0 0.0 0 0)
    (else
      (Audio|PlaySound2D "/Game/Audio/white_death.white_death" 1.0 1.0 0.0 0 0))))